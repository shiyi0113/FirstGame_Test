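; BP_GameEnemy is an enemy that attacks the player while the player is within its attack range.
; On BeginPlay it picks a random skeletal mesh from its Meshes array for visual variety.
; AttackBox overlap events filter for GamePlayer and set a BoxIsOverlapping flag.
; Tick polls that flag and calls Attack every frame while it is set, with no rate limiting in this graph.
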(event OnComponentBeginOverlap(AttackBox)
  (params (OverlappedComponent :type Primitive%20Component%20Object%20Reference) (OtherActor :type Actor%20Object%20Reference) (OtherComp :type Primitive%20Component%20Object%20Reference) (OtherBodyIndex :type Integer) (bFromSweep :type Boolean) (SweepResult :type Hit%20Result%20Structure%20%28by%20ref%29))
  (Utilities|Casting|CastToGamePlayer OtherActor)
  (Variables|Default|SetBoxIsOverlapping true))

(event OnComponentEndOverlap(AttackBox)
  (params (OverlappedComponent :type Primitive%20Component%20Object%20Reference) (OtherActor :type Actor%20Object%20Reference) (OtherComp :type Primitive%20Component%20Object%20Reference) (OtherBodyIndex :type Integer))
  (Utilities|Casting|CastToGamePlayer OtherActor)
  (Variables|Default|SetBoxIsOverlapping false))

(event EventBeginPlay
  (Components|SkeletalMesh|SetSkeletalMeshAsset (Variables|Character|GetMesh) (.OutItem (Utilities|Array|Random (Variables|Default|GetMeshes)))))

(event EventTick
  (params (DeltaSeconds :type Float%20%28single-precision%29))
  (if (Variables|Default|GetBoxIsOverlapping)
    (Class|GameEnemy|Attack)))

(fn ConstructionScript)